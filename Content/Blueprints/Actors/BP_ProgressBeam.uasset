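; BP_ProgressBeam is a beam actor that visualizes wait and track timing by setting a "Progress" scalar parameter on its mesh materials.
; It binds to first-person game mode events, resetting on game start and storing the timer and duration supplied when a wait starts.
; Tick fills the beam from that timer's elapsed time; track start clears the timer.
; Track end starts a local timer of the same duration that drains it.
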(event Custom|OnTrackStarted_Event
  (Utilities|Time|ClearandInvalidateTimerbyHandle (Variables|Default|GetTimer)))

(event Custom|OnTrackEnded_Event
  (bind _returnvalue (Utilities|Time|SetTimerbyEvent (delegate Custom|OnTimerEnded) (Variables|Default|GetDuration)))
  (Variables|Default|SetTimer _returnvalue)
  (Variables|Default|SetProgressFillUp false))

(event Custom|OnTimerEnded
  (Utilities|Time|ClearandInvalidateTimerbyHandle (Variables|Default|GetTimer)))

(event Custom|OnGameStarted_Event
  (CallFunction|SetProgress 0.0))

(event Custom|OnWaitStarted_Event
  (params (Timer :type Timer%20Handle%20Structure) (Duration :type Float%20%28double-precision%29))
  (Variables|Default|SetTimer Timer)
  (Variables|Default|SetDuration Duration)
  (Variables|Default|SetProgressFillUp true))

(event EventBeginPlay
  (CallFunction|SetProgress 0.0)
  (bind _output_get (Variables|Default|SetBP%20First%20Person%20Game%20Mode (CallFunction|GetFirstPersonGameMode)))
  (EventDispatchers|AssignOnGameStarted _output_get (delegate Custom|OnGameStarted_Event))
  (EventDispatchers|AssignOnWaitStarted (Variables|Default|GetBP%20First%20Person%20Game%20Mode) (delegate Custom|OnWaitStarted_Event))
  (EventDispatchers|AssignOnTrackStarted (Variables|Default|GetBP%20First%20Person%20Game%20Mode) (delegate Custom|OnTrackStarted_Event))
  (EventDispatchers|AssignOnTrackEnded (Variables|Default|GetBP%20First%20Person%20Game%20Mode) (delegate Custom|OnTrackEnded_Event)))

(event EventTick
  (params (DeltaSeconds :type Float%20%28single-precision%29))
  (bind _timer (Variables|Default|GetTimer))
  (if (Utilities|Time|IsValidTimerHandle (Variables|Default|GetTimer))
    (CallFunction|SetProgress (/ (select (Variables|Default|GetProgressFillUp) (Class|KismetSystemLibrary|GetTimerElapsedTimeHandle _timer) (Utilities|Time|GetTimerRemainingTimebyHandle _timer)) (Variables|Default|GetDuration)))))

(fn ConstructionScript)

(fn SetProgress
  (params (Value :type Float%20%28double-precision%29))
  (Rendering|Material|SetScalarParameterValueonMaterials (Variables|Debug|GetStaticMeshComponent) "Progress" Value))