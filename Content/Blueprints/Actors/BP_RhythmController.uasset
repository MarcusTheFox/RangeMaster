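; BP_RhythmController is an actor that drives a rhythm game, firing spawners in time with a music track.
; On BeginPlay it caches all BP_Spawner actors sorted by label and the row names of DT_Beatmap.
; Audio playback percent becomes elapsed seconds, triggering the next beat row's spawner by ID with its shot power once its time passes.
; StartPlaying restarts track and beat index; OnTrackFinished fires three seconds after audio ends.
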(event OnAudioPlaybackPercent(AudioCurveSource)
  (params (PlayingSoundWave :type Sound%20Wave%20Object%20Reference) (PlaybackPercent :type Float%20%28single-precision%29))
  (CallFunction|ShotTargetbyAudio (CallFunction|GetAudioElapsedTime PlayingSoundWave PlaybackPercent)))

(event OnAudioFinished(AudioCurveSource)
  (Utilities|FlowControl|Delay 3.0)
  (Default|CallOnTrackFinished))

(event EventBeginPlay
  (bind _outactors (Actor|GetAllActorsOfClass "/Game/Blueprints/Actors/BP_Spawner.BP_Spawner_C"))
  (bind _output_get (Variables|Default|SetSpawners _outactors))
  (Class|GameFunctionLibrary|SortActorArraybyLabel _output_get true)
  (bind _outrownames (DataTable|GetDataTableRowNames "/Game/Data/DT_Beatmap.DT_Beatmap"))
  (Variables|Default|SetRowNames _outrownames))

(fn ConstructionScript)

(fn HasNextBeatEvent
  (return (< (Variables|Default|GetNextBeatEventIndex) (Utilities|Array|Length (Variables|Default|GetRowNames)))))

(fn GetAudioElapsedTime
  (params (PlayingSoundWave :type Sound%20Base%20Object%20Reference) (PlaybackPercent :type Float%20%28single-precision%29))
  (return (* PlaybackPercent (Variables|/Script/Engine.SoundBase|GetDuration PlayingSoundWave))))

(fn ShotTargetbyAudio
  (params (AudioElapsedTime :type Float%20%28double-precision%29))
  (if (CallFunction|HasNextBeatEvent)
    (bind _returnvalue (Utilities|GetDataTableRow "/Game/Data/DT_Beatmap.DT_Beatmap" (Utilities|Array|Get(acopy) (Variables|Default|GetRowNames) (Variables|Default|GetNextBeatEventIndex)))
      (:then
        (if (> AudioElapsedTime (.time _returnvalue))
          (Default|Spawn (Utilities|Array|Get(acopy) (Variables|Default|GetSpawners) (.spawnerid _returnvalue)) (.shotpower _returnvalue))
          (Math|Integer|IncrementInt (Variables|Default|GetNextBeatEventIndex))
          (else
            (return)))))
    (else
      (return))))

(fn StartPlaying
  (Variables|Default|SetNextBeatEventIndex 0)
  (Audio|Components|Audio|Play (Variables|Default|GetAudioCurveSource) 0.0))

(fn GetMaxBeats
  (return (Utilities|Array|Length (Variables|Default|GetRowNames))))