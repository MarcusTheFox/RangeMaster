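; BP_Wall is a wall actor that can be removed or added back with a material dissolve effect.
; RemoveWall and AddWall each play their own timeline to drive the mesh's DissolveAmount parameter, with AddWall negating its track value.
; Timeline updates disable collision during removal and restore query and physics collision during addition.
; Event dispatchers signal the start and completion of each transition.
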(event Custom|RemoveWall
  (Default|CallOnStartRemove)
  (bind _dissolvetrack (Timeline|Timeline PlayFromStart)
    (:Update
      (Rendering|Material|SetScalarParameterValueonMaterials (Variables|Debug|GetStaticMeshComponent) "DissolveAmount" _dissolvetrack)
      (Collision|SetCollisionEnabled (Variables|Debug|GetStaticMeshComponent) "NoCollision"))
    (:Finished
      (Default|CallOnRemoved))))

(event Custom|AddWall
  (Default|CallOnStartAdd)
  (bind _dissolvetrack (Timeline|Timeline_0 PlayFromStart)
    (:Update
      (Rendering|Material|SetScalarParameterValueonMaterials (Variables|Debug|GetStaticMeshComponent) "DissolveAmount" (* _dissolvetrack -1.0))
      (Collision|SetCollisionEnabled (Variables|Debug|GetStaticMeshComponent) "QueryAndPhysics"))
    (:Finished
      (Default|CallOnAdded))))

(fn ConstructionScript)