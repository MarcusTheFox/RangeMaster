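; BP_Target is a hittable target actor that awards combo and score, then dissolves.
; GetHit raises the combo on the game mode's ACScoreSystem, adds BaseScore scaled by the combo multiplier, and reports the hit to the game mode.
; It then switches the cube to physics-only collision while a timeline animates the material's DissolveAmount parameter, destroying the actor when finished.
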(event Custom|DestroyTarget
  (Collision|SetCollisionEnabled (Variables|Default|GetCube) "PhysicsOnly")
  (bind _dissolvetrack (Timeline|DestroyTargetMaterial PlayFromStart)
    (:Update
      (Rendering|Material|SetScalarParameterValueonMaterials (Variables|Default|GetCube) "DissolveAmount" _dissolvetrack))
    (:Finished
      (Actor|DestroyActor))))

(event EventGetHit
  (CallFunction|IncreaseCombo)
  (CallFunction|IncreaseScore)
  (Default|AddHit (CallFunction|GetFirstPersonGameMode) "NewEnumerator0")
  (CallFunction|DestroyTarget))

(event EventBeginPlay
  (bind _output_get (Variables|Default|SetBP%20First%20Person%20Game%20Mode (CallFunction|GetFirstPersonGameMode)))
  (Variables|Default|SetAC%20Score%20System (Variables|/Game/FirstPerson/Blueprints/BP_FirstPersonGameMode.BP_FirstPersonGameMode_C|GetAC_ScoreSystem _output_get)))

(fn ConstructionScript)

(fn IncreaseScore
  (Class|ACScoreSystem|AddScore (Variables|Default|GetAC%20Score%20System) (* (Variables|Default|GetBaseScore) (Default|GetComboMultiplier (Variables|Default|GetBP%20First%20Person%20Game%20Mode)))))

(fn IncreaseCombo
  (Class|ACScoreSystem|IncreaseCombo (Variables|Default|GetAC%20Score%20System) 1))