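; BP_GameStatUI is an actor that shows game UI through a widget component in the range game.
; On BeginPlay it creates the track info and game stat widgets and binds to the RangeMaster game mode's events.
; When the prepare phase starts it displays WB_TrackInfo, and when the game finishes it switches to WB_GameStat.
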(event Custom|OnPreparePhaseStarted_Event
  (UserInterface|SetWidget (Variables|Default|GetWidget) (Variables|Default|GetWB_TrackInfo)))

(event Custom|OnGameFinished_Event
  (params (Result :type Game%20Result%20Data%20Structure%20%28by%20ref%29))
  (UserInterface|SetWidget (Variables|Default|GetWidget) (Variables|Default|GetWB_GameStat)))

(event EventBeginPlay
  (Utilities|FlowControl|Sequence
    (:then_0
      (bind _returnvalue (UserInterface|CreateWidget "/Game/UI/Boards/WB_GameStat.WB_GameStat_C"))
      (Variables|Default|SetWB_GameStat _returnvalue))
    (:then_1
      (bind _returnvalue_2 (UserInterface|CreateWidget "/Game/UI/Boards/WB_TrackInfo.WB_TrackInfo_C"))
      (Variables|Default|SetWB_TrackInfo _returnvalue_2))
    (:then_2
      (Variables|Default|SetRangeMasterGameMode (Class|GameFunctionLibrary|GetRangeMasterGameMode)))
    (:then_3
      (EventDispatchers|AssignOnPreparePhaseStarted (Variables|Default|GetRangeMasterGameMode) (delegate Custom|OnPreparePhaseStarted_Event))
      (EventDispatchers|BindEventtoOnGameFinished (Variables|Default|GetRangeMasterGameMode) (delegate Custom|OnGameFinished_Event)))))

(fn ConstructionScript)