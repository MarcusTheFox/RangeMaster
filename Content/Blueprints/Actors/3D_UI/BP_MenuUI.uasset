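; BP_MenuUI is a 3D UI actor that shows the track start menu in the range game.
; On BeginPlay it gets the RangeMaster game mode, creates a WB_TrackStart widget and assigns it to its Widget component.
; It binds the widget's back button click to force-stop the game through that game mode.
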(event EventBeginPlay
  (Variables|Default|SetGameMode (Class|GameUtilityFunctionLibrary|GetRangeMasterGameMode))
  (bind _returnvalue (UserInterface|CreateWidget "/Game/UI/Boards/WB_TrackStart.WB_TrackStart_C"))
  (bind _output_get (Variables|Default|SetWB_TrackStart _returnvalue))
  (UserInterface|SetWidget (Variables|Default|GetWidget) _output_get)
  (|AssignTrackForceStop))

(fn ConstructionScript)

(event Custom|OnClicked_Event_2
  (Class|RangeMasterGameMode|ForceStopGame (Variables|Default|GetGameMode)))