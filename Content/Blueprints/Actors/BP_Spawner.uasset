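; BP_Spawner is an actor that launches BP_Target actors and registers the ones that go unhit as misses.
; Spawn creates a target 200 units above the spawner and applies an upward velocity-change impulse to its cube, scaled by ShotPower.
; When a target overlaps the Plane component, it is destroyed, a Miss is added to the first-person game mode and the score system's combo resets.
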(event OnComponentBeginOverlap(Plane)
  (params (OverlappedComponent :type Primitive%20Component%20Object%20Reference) (OtherActor :type Actor%20Object%20Reference) (OtherComp :type Primitive%20Component%20Object%20Reference) (OtherBodyIndex :type Integer) (bFromSweep :type Boolean) (SweepResult :type Hit%20Result%20Structure%20%28by%20ref%29))
  (bind _bp_first_person_game_mode (CallFunction|GetFirstPersonGameMode))
  (bind _asbp_target (Utilities|Casting|CastToBP_Target OtherActor))
  (Default|DestroyTarget _asbp_target)
  (Default|AddHit _bp_first_person_game_mode "Miss")
  (Class|ACScoreSystem|ResetCombo (Variables|/Game/FirstPerson/Blueprints/BP_FirstPersonGameMode.BP_FirstPersonGameMode_C|GetAC_ScoreSystem _bp_first_person_game_mode)))

(fn ConstructionScript)

(fn Spawn
  (params (ShotPower :type Integer))
  (bind _returnvalue (Transformation|GetActorTransform))
  (bind _returnvalue_2 (Game|SpawnActorfromClass "/Game/Blueprints/Actors/BP_Target.BP_Target_C" (Math|Transform|MakeTransform (+ (.location _returnvalue) "0.000000,0.000000,200.000000") (.rotation _returnvalue) (.scale _returnvalue)) "Undefined" "MultiplyWithRoot" 0 0))
  (Physics|AddImpulse (Variables|/Game/Blueprints/Actors/BP_Target.BP_Target_C|GetCube _returnvalue_2) (Math|Vector|MakeVector 0.0 0.0 (Math|Conversions|ToFloat(Integer) ShotPower)) "None" true))