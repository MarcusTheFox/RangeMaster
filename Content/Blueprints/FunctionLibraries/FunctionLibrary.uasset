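; Blueprint function library of shared helpers for a first-person game.
; Two getters cast the game mode and player zero's controller to the project's first-person classes, printing a red error on screen if the cast fails.
; A formatting helper turns a seconds count into minutes:seconds text with zero-padded seconds.
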(fn GetFirstPersonGameMode
  (bind _asbp_first_person_game_mode (Utilities|Casting|CastToBP_FirstPersonGameMode (Game|GetGameMode))
    (:then
      (return _asbp_first_person_game_mode))
    (:CastFailed
      (Development|PrintString 0 "Game mode cast fail!" true true "(R=1.000000,G=0.000000,B=0.000000,A=1.000000)"))))

(fn GetFirstPersonController
  (bind _asbp_first_person_player_controller (Utilities|Casting|CastToBP_FirstPersonPlayerController (Game|GetPlayerController 0))
    (:then
      (return _asbp_first_person_player_controller))
    (:CastFailed
      (Development|PrintString 0 "Player controller cast fail!" true true "(R=1.000000,G=0.000000,B=0.000000,A=1.000000)"))))

(fn FormatTime
  (params (TotalSeconds :type Float%20%28double-precision%29))
  (return (Utilities|Text|FormatText "{mm}:{ss}" (Math|Float|Floor (/ TotalSeconds 6e+01)) (Utilities|Text|ToText(Integer) (Math|Float|Floor (Math|Float|%(Float) TotalSeconds 6e+01)) false true 2))))