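; Game instance that saves and loads the player's best result for each track.
; SaveResult writes a new BP_SaveGame to a slot named after the track ID, but only when no ranked result exists or the new max score is higher.
; LoadResult reads that slot and falls back to a zero score with no rank when no valid save is found.
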(fn SaveResult
  (params (TrackID :type Name) (TrackResult :type S%20Track%20Result%20Structure))
  (LocalVariables|SetL_TrackID TrackID)
  (LocalVariables|SetL_TrackResult TrackResult)
  (bind _trackresult (CallFunction|LoadResult (LocalVariables|GetL_TrackID)))
  (if (Utilities|Enum|NotEqual(Enum) (.rank _trackresult) "None")
    (if (< (.maxscore _trackresult) (.MaxScore (Utilities|Struct|BreakS_TrackResult (LocalVariables|GetL_TrackResult))))
      _
      (else
        (return))))
  (bind _returnvalue (SaveGame|CreateSaveGameObject "/Game/Blueprints/SaveGame/BP_SaveGame.BP_SaveGame_C"))
  (Default|SaveResult _returnvalue (LocalVariables|GetL_TrackResult))
  (SaveGame|SaveGametoSlot _returnvalue (Utilities|String|ToString(Name) (LocalVariables|GetL_TrackID))))

(fn LoadResult
  (params (TrackID :type Name))
  (bind _returnvalue (SaveGame|LoadGamefromSlot (Utilities|String|ToString(Name) TrackID)))
  (bind _asbp_save_game (Utilities|Casting|CastToBP_SaveGame _returnvalue)
    (:then
      (return (Variables|/Game/Blueprints/SaveGame/BP_SaveGame.BP_SaveGame_C|GetTrackResult _asbp_save_game)))
    (:CastFailed
      (return (Utilities|Struct|MakeS_TrackResult 0 "None")))))